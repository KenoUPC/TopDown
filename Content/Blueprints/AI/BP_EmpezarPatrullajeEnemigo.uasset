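; Zone trigger actor that assigns and clears the target of a group of enemies as the player enters and leaves.
; Overlapping actors are identified as the player by checking for the BPI_PLayer interface.
; On begin overlap, each enemy in EnemigosZona1 receives a SetTarget message with that actor, and on end overlap the same message with an empty target.
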(event `self.ReceiveBeginPlay`)

(event `self.ReceiveActorBeginOverlap`
  (params (OtherActor :type "Actor Object Reference"))
  (if (`KismetSystemLibrary.DoesImplementInterface` OtherActor "/Game/Blueprints/Interfaces/BPI_PLayer.BPI_PLayer_C")
    (for _array_element (`self.EnemigosZona1`)
      (message `/Game/Blueprints/Interfaces/BPI_Enemigo.SetTarget` _array_element OtherActor))))

(event `self.ReceiveActorEndOverlap`
  (params (OtherActor :type "Actor Object Reference"))
  (if (`KismetSystemLibrary.DoesImplementInterface` OtherActor "/Game/Blueprints/Interfaces/BPI_PLayer.BPI_PLayer_C")
    (for _array_element (`self.EnemigosZona1`)
      (message `/Game/Blueprints/Interfaces/BPI_Enemigo.SetTarget` _array_element null))))

(fn `UserConstructionScript`)