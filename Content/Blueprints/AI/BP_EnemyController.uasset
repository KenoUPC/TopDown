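; BP_EnemyController is an AI controller that runs the BT_Enemy behavior tree for an enemy.
; On possess it starts the tree and writes a zero vector to a Blackboard key, and on BeginPlay it prints a debug string.
; Unconnected leftover nodes for look-at direction, activation and a BP_Hero player cast never execute.
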(event `self.ReceiveTick`
  (params (DeltaSeconds :type "Float (single-precision)")))

(event `self.ReceivePossess`
  (params (PossessedPawn :type "Pawn Object Reference"))
  (`self.RunBehaviorTree` "/Game/Blueprints/AI/BT_Enemy.BT_Enemy")
  (`BlackboardComponent.SetValueAsVector` (`self.Blackboard`) (`self.Key Name`) (0.0 0.0 0.0)))

(event `self.ReceiveBeginPlay`
  (`KismetSystemLibrary.PrintString` "AI_ACtivada"))

(fn `UserConstructionScript`)