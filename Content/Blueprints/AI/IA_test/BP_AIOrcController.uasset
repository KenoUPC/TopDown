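; AI controller for an orc enemy that tracks the player hero through AI perception.
; On possess it runs the BT_Orc behavior tree.
; Perception updates for BP_Hero store the hero in a blackboard object key when sensed and empty that key when lost, printing a Spanish debug message each time.
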(event `self.ReceivePossess`
  (params (PossessedPawn :type "Pawn Object Reference"))
  (`self.RunBehaviorTree` "/Game/Blueprints/AI/IA_test/BT_Orc.BT_Orc"))

(event `self.AIPerception.OnTargetPerceptionUpdated`
  (params (Actor :type "Actor Object Reference") (Stimulus :type "AIStimulus Structure"))
  (bind _asbp_hero (cast `/Game/Blueprints/Characters/Hero/BP_Hero` Actor))
  (if Stimulus_bSuccessfullySensed
    (`BlackboardComponent.SetValueAsObject` (`AIBlueprintHelperLibrary.GetBlackboard` null) (`self.Key Name`) _asbp_hero)
    (`KismetSystemLibrary.PrintString` "VI al Objetivo")
    (else
      (`BlackboardComponent.SetValueAsObject` (`AIBlueprintHelperLibrary.GetBlackboard` null) (`self.Key Name`) null)
      (`KismetSystemLibrary.PrintString` "deje de verlo"))))

(fn `UserConstructionScript`)