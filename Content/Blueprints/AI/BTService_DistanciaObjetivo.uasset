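; Behavior tree service that records the distance from the AI-controlled pawn to its combat target in a blackboard float.
; It runs on activation only, with no tick logic, reading the target actor key and writing GetDistanceTo's result to the distance key.
; For debugging, it prints both a vector-based distance and the GetDistanceTo value, and draws a short-lived arrow from pawn to target.
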(event `self.ReceiveActivationAI`
  (params (OwnerController :type "AIController Object Reference") (ControlledPawn :type "Pawn Object Reference"))
  (bind _returnvalue (`Actor.K2_GetActorLocation` ControlledPawn))
  (bind _returnvalue_2 (`BTFunctionLibrary.GetBlackboardValueAsActor` (`self.BBKey_CombatTarget`)))
  (bind _returnvalue_3 (`Actor.K2_GetActorLocation` _returnvalue_2))
  (bind _returnvalue_4 (`Actor.GetDistanceTo` ControlledPawn _returnvalue_2))
  (`KismetSystemLibrary.PrintString` (`KismetStringLibrary.Concat_StrStr` "Calculo con vector" (`KismetStringLibrary.Conv_DoubleToString` (`KismetMathLibrary.Vector_Distance` _returnvalue _returnvalue_3))) true true (struct :`R` 1.0 :`G` 0.15625 :`B` 0.15625 :`A` 1.0))
  (`KismetSystemLibrary.PrintString` (`KismetStringLibrary.Conv_DoubleToString` _returnvalue_4))
  (`BTFunctionLibrary.SetBlackboardValueAsFloat` (`self.BBKey_Distancia`) _returnvalue_4)
  (`KismetSystemLibrary.DrawDebugArrow` _returnvalue _returnvalue_3 25.0 (struct :`R` 0.12946 :`G` 1.0 :`B` 0.109634 :`A` 1.0) 5.0))