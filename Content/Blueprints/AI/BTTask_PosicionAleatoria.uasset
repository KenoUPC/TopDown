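; Behavior Tree task that picks a random position near the AI-controlled pawn and stores it in the Blackboard.
; On execute, it takes X and Y from a random reachable navigation point within a fixed radius, keeping the pawn's current Z.
; It writes the vector to the BBKeyPosicion key and finishes successfully without moving the pawn.
; A debug sphere draw for the location is left unconnected.
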(event `self.ReceiveExecuteAI`
  (params (OwnerController :type "AIController Object Reference") (ControlledPawn :type "Pawn Object Reference"))
  (bind _returnvalue (`Actor.K2_GetActorLocation` ControlledPawn))
  (bind _output_get (set `self.Random Location` (`KismetMathLibrary.MakeVector` (.x (`NavigationSystemV1.K2_GetRandomReachablePointInRadius` _returnvalue 400.0 null null)) (.y (`NavigationSystemV1.K2_GetRandomReachablePointInRadius` _returnvalue 400.0 null null)) (.z _returnvalue))))
  (`BTFunctionLibrary.SetBlackboardValueAsVector` (`self.BBKey_posicion`) (`self.Random Location`))
  (`self.FinishExecute` true))