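; BP_Hero is the player hero for top-down play, handling movement, the HUD and damage display.
; BeginPlay adds the IMC_TopDown Enhanced Input context and creates the overlay widget.
; IA_Move stores the direction and moves along world X/Y axes, while Tick prints the forward vector for debugging.
; AnyDamage calls the empty DañoRecibido stub, then refreshes the health widget, so health is unchanged in this graph.
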(event `self.ReceiveBeginPlay`
  (`self.AddMaping`)
  (`self.Create UI`))

(event `self.ReceiveAnyDamage`
  (params (Damage :type "Float (single-precision)") (DamageType :type "DamageType Object Reference") (InstigatedBy :type "Controller Object Reference") (DamageCauser :type "Actor Object Reference"))
  (`self.DañoRecibido` Damage)
  (`/Game/Blueprints/Widgets/WBP_SaludJugador.UpdateSaludPlayerUI` (`/Game/Blueprints/Widgets/WBP_Overlay.WBP_SaludJugador` (`self.Overlay`)) (`self.Saludactual`) (`self.SaludMaxima`)))

(event `self.ReceiveTick`
  (params (DeltaSeconds :type "Float (single-precision)"))
  (`KismetSystemLibrary.PrintString` (`KismetStringLibrary.Conv_VectorToString` (`self.GetActorForwardVector`)) true true (struct :`G` 0.66 :`B` 1.0 :`A` 1.0) 2.0 "1"))

(event `EnhancedInput|/Game/Blueprints/Characters/Input/Action/IA_Move`
  (params (ActionValue :type "Vector2D Structure") (ElapsedSeconds :type "Float (double-precision)") (TriggeredSeconds :type "Float (double-precision)") (InputAction :type "InputAction Object Reference" :default "/Game/Blueprints/Characters/Input/Action/IA_Move.IA_Move"))
  (bind (_x _y) (`KismetMathLibrary.BreakVector2D` ActionValue))
  (:`Triggered`
    (set `self.Direccion` ActionValue)
    (`self.AddMovementInput` (1.0 0.0 0.0) _x)
    (`self.AddMovementInput` (0.0 1.0 0.0) _y)))

(fn `AddMaping`
  (bind _asplayer_controller (cast `PlayerController` (`self.GetController`)))
  (`EnhancedInputSubsystemInterface.AddMappingContext` (pcsubsystem `EnhancedInputLocalPlayerSubsystem` _asplayer_controller) "/Game/Blueprints/Characters/Input/MapingContext/IMC_TopDown.IMC_TopDown" 0 (struct)))

(fn `Create UI`
  (bind _returnvalue (`|CreateWidget` "/Game/Blueprints/Widgets/WBP_Overlay.WBP_Overlay_C" (cast `PlayerController` (`self.GetController`) :!pure true)))
  (bind _output_get (set `self.Overlay` _returnvalue))
  (`UserWidget.AddToViewport` _output_get 0))

(fn `DañoRecibido`
  (params (`Daño` :type "Float (double-precision)")))

(fn `UserConstructionScript`
  (`parent.UserConstructionScript`))