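; Orc enemy character that sets its AI target, plays attacks and shows health on a widget.
; SetTarget writes the given object to the controller's Blackboard target key.
; Ataque plays the attack as a PaperZD animation override, using EstaAtacando to block re-triggering until it completes or is cancelled.
; SeBajoVIda passes current and maximum health to the WBP_VidaEnemigo widget when health drops.
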(event `self.ReceiveBeginPlay`
  (`parent.ReceiveBeginPlay`))

(event `self.ReceiveTick`
  (params (DeltaSeconds :type "Float (single-precision)"))
  (`parent.ReceiveTick` 0.0))

(event `/Game/Blueprints/Interfaces/BPI_Enemigo.SetTarget`
  (params (Objetivo :type "Actor Object Reference"))
  (`BlackboardComponent.SetValueAsObject` (`AIBlueprintHelperLibrary.GetBlackboard` (`self.GetController`)) (`self.TargetBBKeyName`) Objetivo))

(event `/Game/Blueprints/Interfaces/BPI_Enemigo.Ataque`
  (if (not (`self.bEstaAtacando?`))
    (`PaperZDPlaySlotOverrideAction.PlayAnimationOverrideWithCallbacks` (`PaperZDAnimationComponent.AnimInstance` (`self.AnimationComponent`)) "/Game/Blueprints/Characters/Enemy/Anim/AnimSequences/Attack.Attack"
      (:`then`
        (set `self.bEstaAtacando?` true))
      (:`OnCompleted`
        (set `self.bEstaAtacando?` false :!label _label))
      (:`OnCancelled`
        (goto _label)))))

(event `self.SeBajoVIda`
  (params (VidaActual :type "Float (double-precision)") (VidaMaxima :type "Float (double-precision)"))
  (bind _aswbp_vida_enemigo (cast `/Game/Blueprints/Widgets/WBP_VidaEnemigo` (`WidgetComponent.GetWidget` (`self.Widget`))))
  (`/Game/Blueprints/Widgets/WBP_VidaEnemigo.Update` _aswbp_vida_enemigo VidaActual VidaMaxima))

(fn `UserConstructionScript`
  (`parent.UserConstructionScript`))