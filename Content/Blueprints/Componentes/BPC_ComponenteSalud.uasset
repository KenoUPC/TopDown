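; BPC_ComponenteSalud is a health component that tracks current health and a death flag.
; DisminuirVida subtracts incoming damage, takes the Min with zero, so the result never exceeds zero, and sets EstaMuerto from it.
; AumentarVida adds health and takes the Max with VidaMaxima, so the result never falls below maximum.
; Both functions print debug messages, and the event graph has no active logic.
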(fn `AumentarVida`
  (params (VidaEntrante :type "Float (double-precision)"))
  (set `self.VidaActual` (`KismetMathLibrary.FMax` (+ (`self.VidaActual`) VidaEntrante) (`self.VidaMaxima`)))
  (`KismetSystemLibrary.PrintString` "se aumento vida"))

(fn `DisminuirVida`
  (params (`DañoEntrante` :type "Float (double-precision)"))
  (set `self.VidaActual` (`KismetMathLibrary.FMin` (- (`self.VidaActual`) `DañoEntrante`)))
  (set `self.bEstaMuerto?` (<= (`self.VidaActual`) 0.0))
  (`KismetSystemLibrary.PrintString` "Se quito vida"))