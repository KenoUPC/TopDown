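; BP_GIPlayer is a Game Instance Blueprint that holds the player's save data object.
; On Init it loads SG_Data from the named slot if one exists, otherwise it creates a new one.
; Guardar passes a struct to that object and prints a confirmation, without writing the slot to disk here.
; GetSave returns the stored data from the same object.
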(event `self.ReceiveInit`
  (bind _returnvalue (`GameplayStatics.DoesSaveGameExist` (`self.Slot Name`) 2))
  (if _returnvalue
    (bind _returnvalue_2 (`GameplayStatics.LoadGameFromSlot` (`self.Slot Name`) 2))
    (bind _assg_data (cast `/Game/Blueprints/Save/SG_Data` _returnvalue_2))
    (bind _output_get (set `self.SaveG` _assg_data))
    (else
      (bind _returnvalue_3 (`GameplayStatics.CreateSaveGameObject` "/Game/Blueprints/Save/SG_Data.SG_Data_C"))
      (set `self.SaveG` _returnvalue_3))))

(fn `GetSave`
  (returns (Struct :type "/Game/Blueprints/Struct/S_estructuraSave Structure"))
  (bind _newparam (`/Game/Blueprints/Save/SG_Data.GetSave` (`self.SaveG`)))
  (return _newparam))

(fn `Guardar`
  (params (Struct :type "/Game/Blueprints/Struct/S_estructuraSave Structure"))
  (`/Game/Blueprints/Save/SG_Data.Set Struct` (`self.SaveG`) Struct)
  (`KismetSystemLibrary.PrintString` "Se guardo la estructura"))