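; BP_GIKnight is a game instance that saves and loads a stored transform through a BP_SaveGame object.
; On Init it loads the save from the named slot, or creates a new save object if none exists.
; Guardar1 stores a given transform and writes it to the slot through Guardar, while Cargar returns the transform held in the cached save object.
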(event `self.ReceiveInit`
  (bind _returnvalue (`GameplayStatics.DoesSaveGameExist` (`self.Slot Name`)))
  (if _returnvalue
    (bind _returnvalue_2 (`GameplayStatics.LoadGameFromSlot` (`self.Slot Name`)))
    (bind _asbp_save_game (cast `/Game/Blueprints/Game/BP_SaveGame` _returnvalue_2))
    (set `self.SaveGame` _asbp_save_game)
    (else
      (bind _returnvalue_3 (`GameplayStatics.CreateSaveGameObject` "/Game/Blueprints/Game/BP_SaveGame.BP_SaveGame_C"))
      (set `self.SaveGame` _returnvalue_3))))

(event `Guardar`
  (`GameplayStatics.SaveGameToSlot` (`self.SaveGame`) (`self.Slot Name`)))

(fn `cargar`
  (returns (NewParam :type "Transform Structure"))
  (return (`/Game/Blueprints/Game/BP_SaveGame.Transform` (`self.SaveGame`))))

(fn `Guardar1`
  (params (Transform :type "Transform Structure"))
  (set `/Game/Blueprints/Game/BP_SaveGame.Transform` Transform (`self.SaveGame`))
  (`self.Guardar`))