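; BP_GIKnight is a game instance that persists a saved transform through a SaveGame object.
; On Init it loads the existing save slot or creates a new save object.
; Guardar1 stores a transform and writes it to the slot via Guardar, while Cargar returns the transform held in memory.
; Debug keys O and L, also in this graph, save and restore an actor transform through the game instance.
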(event Custom|Guardar
  (SaveGame|SaveGametoSlot (Variables|Default|GetSaveGame) (Variables|Default|GetSlot%20Name)))

(event EventInit
  (bind _returnvalue (SaveGame|DoesSaveGameExist (Variables|Default|GetSlot%20Name)))
  (if _returnvalue
    (bind _returnvalue_2 (SaveGame|LoadGamefromSlot (Variables|Default|GetSlot%20Name)))
    (bind _asbp_save_game (Utilities|Casting|CastTo _returnvalue_2))
    (Variables|Default|SetSaveGame _asbp_save_game)
    (else
      (bind _returnvalue_3 (SaveGame|CreateSaveGameObject))
      (Variables|Default|SetSaveGame _returnvalue_3))))

(event Input|KeyboardEvents|DebugKeyL
  (params (Key :type Key%20Structure :default "None") (ActionValue :type Input%20Action%20Value%20Structure))
  (:Released
    (bind _asbp_giknight (Utilities|Casting|CastToBP_GIKnight (Game|GetGameInstance)))
    (bind _newparam (CallFunction|Cargar _asbp_giknight))
    (Transformation|SetActorTransform _newparam)))

(event Input|KeyboardEvents|DebugKeyO
  (params (Key :type Key%20Structure :default "None") (ActionValue :type Input%20Action%20Value%20Structure))
  (:Released
    (bind _asbp_giknight (Utilities|Casting|CastToBP_GIKnight (Game|GetGameInstance)))
    (CallFunction|Guardar1 _asbp_giknight (Transformation|GetActorTransform))))

(fn Guardar1
  (params (Transform :type Transform))
  (Variables|Default|SetTransform (Variables|Default|GetSaveGame) Transform)
  (CallFunction|Guardar))

(fn Cargar
  (return (Variables|Default|GetTransform (Variables|Default|GetSaveGame))))